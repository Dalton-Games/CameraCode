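; Player controller for an isometric 3D camera, handling zoom, yaw rotation and view movement.
; Input events accumulate clamped zoom and yaw, switch the cursor while dragging, and track mouse or touch drag state.
; Each Tick pushes yaw and zoom to the controlled camera pawn.
; Dragging moves the view to the traced point under cursor or finger plus eye height; otherwise axis input moves the pawn relative to camera yaw.
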(event `InputAction|CamZoomOut`
  ;[1 1 1] Set Zoom Out
  (:`Pressed`
    (set `self.CameraZoom` (`KismetMathLibrary.FClamp` (+ (`self.CameraZoom`) -0.1)))))

(event `InputAction|CamZoomIn`
  ;[1 1 1] Set Zoom In
  (:`Pressed`
    (set `self.CameraZoom` (`KismetMathLibrary.FClamp` (+ (`self.CameraZoom`) 0.1)))))

(event `InputAxis|CamZoom`
  (params (AxisValue :type "Float (single-precision)"))
  ;[1 1 1] Update Zoom Level from axis
  (set `self.CameraZoom` (`KismetMathLibrary.FClamp` (+ AxisValue (`self.CameraZoom`)))))

(event `InputAxis|CamRotate`
  (params (AxisValue :type "Float (single-precision)"))
  ;[1 1 1] Gets Camera Rotation
  (set `self.CameraYaw` (+ AxisValue (`self.CameraYaw`))))

(event `InputAction|CamDragView` :consume false
  ;[1 1 1] Detect User draging
  (:`Pressed`
    (set `self.MouseDrag` true)
    (set `self.CurrentMouseCursor` "GrabHand"))
  (:`Released`
    (set `self.MouseDrag` false)
    (set `self.CurrentMouseCursor` "Hand")))

(event `InputTouch`
  (params (Location :type "Object.Vector Structure") (FingerIndex :type "InputCoreTypes.ETouchIndex Enum"))
  ;[1 1 1] Detect User draging
  (:`Pressed`
    (set `self.TouchDrag` true))
  (:`Released`
    (set `self.TouchDrag` false)))

(event `self.ReceiveTick`
  (params (DeltaSeconds :type "Float (single-precision)"))
  (bind (_worldlocation _worlddirection) (`self.DeprojectMousePositionToWorld`))
  (bind (_hitresult _returnvalue) (`self.GetHitResultUnderFingerByChannel` "Touch1" "TraceTypeQuery1" false))
  ;[1 1 1] Update Camera Yaw and Zoom
  (bind _asbp_camerapawn_c (`self.GetControledCameraPawn`)
    (:`then`
      (set `self.Camera Pawn` null)
      (set `/Game/Base/BP_Iso3dPlayercontroller.Yaw` (`self.CameraYaw`) _asbp_camerapawn_c)
      (`self.SetCameraZoomLevel` _asbp_camerapawn_c (`self.CameraZoom`))
      (if (`self.MouseDrag`)
        ;[1 1 1] Move Camera by Mouse
        (bind (_outhit _returnvalue_2) (`KismetSystemLibrary.LineTraceSingle` _worldlocation (+ _worldlocation (* _worlddirection 20000.0)) "TraceTypeQuery1"))
        (if _returnvalue_2
          (`self.K2_SetActorLocation` (+ (`GameplayStatics.BreakHitResult` _outhit) (`KismetMathLibrary.MakeVector` 0.0 0.0 (`Pawn.BaseEyeHeight`)))))
        (elif (`self.TouchDrag`)
          ;[1 1 1] Move Camera by Mouse
          (if _returnvalue
            (`self.K2_SetActorLocation` (+ (`GameplayStatics.BreakHitResult` _hitresult) (`KismetMathLibrary.MakeVector` 0.0 0.0 (`Pawn.BaseEyeHeight`)))))
          (else
            ;[1 1 1] Move Camera by Axis
            (`Pawn.AddMovementInput` (`self.GetControlledPawn`) (`KismetMathLibrary.RotateAngleAxis` (`KismetMathLibrary.MakeVector` (`self.GetInputAxisValue`) (`self.GetInputAxisValue`)) (`self.CameraYaw`) (0.0 0.0 1.0)) 1.0)))))))

(fn `UserConstructionScript`
  (set `self.MouseDrag` false)
  (set `self.TouchDrag` false))